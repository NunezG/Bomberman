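; Game mode for a two-player local Bomberman game, handling the menu setup and the transition into a level.
; On BeginPlay it creates the second player, respawns both at ID-matched PlayerStarts with distinct colours, reads tile data and shows the menu.
; The bound LevelStart event spawns blocks, blends to a centred stage camera fitted to the level's aspect ratio, and moves players onto colour-lit spawn blocks, enabling them to start.
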(event `self.ReceiveBeginPlay`
  (bind _returnvalue (`GameplayStatics.GetPlayerController` 0))
  (add `self.StartLevel` (delegate `LevelStart`))
  ;[1 1 1] Create and spawn players in their menu locations
  (`GameplayStatics.CreatePlayer` 1)
  (`self.CorrectPlayerSpawns` (cast `BombermanPlayerController` (`GameplayStatics.GetPlayerController` 0) :!pure true))
  (`self.CorrectPlayerSpawns` (cast `BombermanPlayerController` (`GameplayStatics.GetPlayerController` 1) :!pure true) 1)
  (`self.ReadTileDataFromFile` 1)
  ;[1 1 1] Set Starting camera
  (bind _outactors (`GameplayStatics.GetAllActorsWithTag` "StartCamera"))
  (for _array_element _outactors
    (bind _ascamera_actor (cast `CameraActor` _array_element))
    (`PlayerController.SetViewTargetWithBlend` _returnvalue _ascamera_actor 0.0 "VTBlend_Linear" 0.0 false)
    (bind _returnvalue_2 (`|CreateWidget` "/Game/Blueprints/UI/MenuScreen.MenuScreen_C" _returnvalue))
    (`UserWidget.AddToPlayerScreen` _returnvalue_2 0)))

(event `LevelStart`
  (`self.SpawnBlocks`)
  ;[1 1 1] Setup camera aspect ratio, then move it to the map centre point and set it to the current view
  (bind _outactors (`GameplayStatics.GetAllActorsOfClass` "/Game/Blueprints/BMStageCameraActor_BP.BMStageCameraActor_BP_C"))
  (bind _output (`|GetArrayItem` _outactors))
  (`CameraComponent.SetAspectRatio` (`BMStageCameraActor.StageCamera` _output) (/ (`KismetMathLibrary.Conv_IntToDouble` (`self.levelWidth`)) (`KismetMathLibrary.Conv_IntToDouble` (`self.levelHeight`))))
  (`self.K2_SetActorLocation` _output (`self.mapCenter`) false false)
  (`PlayerController.SetViewTargetWithBlend` (`GameplayStatics.GetPlayerController` 0) _output 1.0 "VTBlend_EaseInOut" 1.0 false)
  ;[1 0.2592 0.2393] Set players to their correct starting positions
  (bind _outactors_2 (`GameplayStatics.GetAllActorsOfClass` "/Game/Blueprints/Blocks/PlayerSpawnBlock.PlayerSpawnBlock_C"))
  (for (_array_element _array_index) _outactors_2
    (bind _returnvalue (`Controller.K2_GetPawn` (`GameplayStatics.GetPlayerController` _array_index)))
    (bind (_returnvalue_x _returnvalue_y _returnvalue_z) (`KismetMathLibrary.BreakVector` (`self.K2_GetActorLocation` _array_element)))
    (`self.K2_SetActorLocation` _returnvalue (`KismetMathLibrary.MakeVector` _returnvalue_x _returnvalue_y (+ _returnvalue_z 500.0)) false false)
    ;[1 1 1] Set light colour in starting areas from player colour
    (bind _asbomberman_character_bp (cast `/Game/TopDownCPP/Blueprints/BombermanCharacter_BP` _returnvalue))
    (`/Game/Blueprints/Blocks/PlayerSpawnBlock.SetLightColour` _array_element (`/Game/TopDownCPP/Blueprints/BombermanCharacter_BP.Player Colour` _asbomberman_character_bp))
    (set `/Game/TopDownCPP/Blueprints/BombermanCharacter_BP.canStart` true _asbomberman_character_bp)))

(fn `CorrectPlayerSpawns`
  (params (PlayerRef :type "BombermanPlayerController Object Reference") (PlayerID :type Integer))
  (bind _returnvalue (`Controller.K2_GetPawn` PlayerRef))
  (`self.K2_DestroyActor` (`Controller.K2_GetPawn` PlayerRef))
  (`self.RestartPlayerAtPlayerStart` PlayerRef (`self.K2_FindPlayerStart` PlayerRef (`KismetStringLibrary.Conv_IntToString` PlayerID)))
  (switch `int` PlayerID
    (:`0`
      (bind _asbomberman_character_bp (cast `/Game/TopDownCPP/Blueprints/BombermanCharacter_BP` _returnvalue))
      (`/Game/TopDownCPP/Blueprints/BombermanCharacter_BP.SetPlayerColour` _asbomberman_character_bp (`KismetMathLibrary.MakeColor` 1.0 0.1)))
    (:`1`
      (bind _asbomberman_character_bp_2 (cast `/Game/TopDownCPP/Blueprints/BombermanCharacter_BP` _returnvalue))
      (`/Game/TopDownCPP/Blueprints/BombermanCharacter_BP.SetPlayerColour` _asbomberman_character_bp_2 (`KismetMathLibrary.MakeColor` 0.0 0.1 1.0)))))

(fn `UserConstructionScript`)