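; Bomb actor Blueprint that handles the visual side of a fuse burning and the bomb exploding.
; On fuse lit, it creates a dynamic material once and starts the Burst timeline, which drives the ColourLerp parameter scaled by FuseTime to shift the bomb's colour.
; On explode, it spawns the explosion emitter at the actor's location and destroys itself.
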(event `self.OnFuseLit`
  (bind _mesh (`self.mesh`))
  ;[1 1 1] Create dynamic instance to change bomb colour at runtime
  (`/Engine/EditorBlueprintResources/StandardMacros.IsValid` (`self.Material`)
    (:`Is Not Valid`
      (bind _returnvalue (`PrimitiveComponent.CreateDynamicMaterialInstance` _mesh 0 (`PrimitiveComponent.GetMaterial` _mesh 0)))
      (`PrimitiveComponent.SetMaterial` _mesh 0 _returnvalue)
      (set `self.Material` _returnvalue)
      ;[1 1 1] Change bomb colour over time
      (bind (_direction _colourlerp) (`Timeline|Burst` :!via `PlayFromStart`)
        (:`Update`
          (`MaterialInstanceDynamic.SetScalarParameterValue` (`self.Material`) "ColourLerp" (/ _colourlerp (`self.fuseTime`))))))))

(event `self.OnExplode`
  (`GameplayStatics.SpawnEmitterAtLocation` (`self.explosion`) (`self.K2_GetActorLocation`))
  (`self.K2_DestroyActor`))

(fn `UserConstructionScript`)